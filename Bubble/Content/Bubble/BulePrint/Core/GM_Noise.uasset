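; Game mode for the Bubble game that manages the start menu, play timer and end-of-game flow.
; Outside TestMap it shows the start UI with a mouse cursor, and StartPlaying opens TestMap as the play level.
; Tick accumulates PlayTime until GameOver.
; gameGG shows a win or lose widget with its sound, destroys the boss, then quits the game after a short delay.
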(event Custom|gameGG
  (params (Win :type Boolean))
  (Variables|Default|SetGameOver true)
  (if Win
    (bind _returnvalue (UserInterface|CreateWidget "/Game/Bubble/BulePrint/UI/win.win_C"))
    (UserInterface|Viewport|AddtoViewport _returnvalue 0)
    (bind _returnvalue_2 (Audio|CreateSound2D "/Game/Bubble/Asset/Audio/胜利音效.胜利音效" 1.0 1.0 0.0 0))
    (Audio|Components|Audio|Play _returnvalue_2 0.0)
    (else
      (bind _returnvalue_3 (UserInterface|CreateWidget "/Game/Bubble/BulePrint/UI/lose.lose_C"))
      (UserInterface|Viewport|AddtoViewport _returnvalue_3 0)
      (bind _returnvalue_4 (Audio|CreateSound2D "/Game/Bubble/Asset/Audio/game_over.game_over" 1.0 1.0 0.0 0))
      (Audio|Components|Audio|Play _returnvalue_4 0.0)))
  (bind _returnvalue_5 (Actor|GetActorOfClass "/Game/Bubble/BulePrint/Boss/BP_Boss.BP_Boss_C"))
  (Utilities|IsValid _returnvalue_5
    (:Is%20Valid
      (Actor|DestroyActor _returnvalue_5))
    (:Is%20Not%20Valid
      _))
  (Utilities|FlowControl|Delay 5.0)
  (Game|QuitGame 0 "Quit" false))

(event Custom|StartPlaying
  (Game|OpenLevel(byName) "TestMap"))

(event EventBeginPlay
  (bind _returnvalue (Game|GetCurrentLevelName true))
  (if (Utilities|Enum|NotEqual(Enum) _returnvalue "TestMap")
    (bind _returnvalue_2 (UserInterface|CreateWidget "/Game/Bubble/BulePrint/UI/StartUI.StartUI_C"))
    (UserInterface|Viewport|AddtoViewport _returnvalue_2 0)
    (Variables|/Script/Engine.PlayerController|SetbShowMouseCursor (Game|GetPlayerController 0) true)))

(event EventTick
  (params (DeltaSeconds :type Float%20%28single-precision%29))
  (if (not (Variables|Default|GetGameOver))
    (Variables|Default|SetPlayTime (+ (Variables|Default|GetPlayTime) DeltaSeconds))))

(fn ConstructionScript)