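; A large bubble projectile that the main character can bounce off or burst, self-expiring after a few seconds.
; Touching the top box grants an extra jump, forces a jump, plays force feedback and destroys the bubble.
; Dashing into the side box replaces it with small bubbles fanned out in pitch.
; A shared Used flag allows one trigger, consumed even by a non-dashing side touch; the construction script selects launch speed.
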(event OnComponentBeginOverlap(SideBox)
  (params (OverlappedComponent :type Primitive%20Component%20Object%20Reference) (OtherActor :type Actor%20Object%20Reference) (OtherComp :type Primitive%20Component%20Object%20Reference) (OtherBodyIndex :type Integer) (bFromSweep :type Boolean) (SweepResult :type Hit%20Result%20Structure%20%28by%20ref%29))
  (bind _asmaincharacter (Utilities|Casting|CastTomaincharacter OtherActor))
  (bind _output_get (Variables|Default|SetAs%20Maincharacter _asmaincharacter))
  (if (not (Variables|Default|GetUsed))
    (Variables|Default|SetUsed true)
    (if (Variables|/Game/Bubble/BulePrint/Core/maincharacter.maincharacter_C|GetDashing _output_get)
      (CallFunction|BubbleBreak false))))

(event OnComponentBeginOverlap(TopBox)
  (params (OverlappedComponent :type Primitive%20Component%20Object%20Reference) (OtherActor :type Actor%20Object%20Reference) (OtherComp :type Primitive%20Component%20Object%20Reference) (OtherBodyIndex :type Integer) (bFromSweep :type Boolean) (SweepResult :type Hit%20Result%20Structure%20%28by%20ref%29))
  (bind _asmaincharacter (Utilities|Casting|CastTomaincharacter OtherActor))
  (Variables|Default|SetAs%20Maincharacter _asmaincharacter)
  (if (not (Variables|Default|GetUsed))
    (Variables|Default|SetUsed true)
    (CallFunction|BubbleBreak true)
    (ForceFeedback|SpawnForceFeedbackAttached "/Game/Bubble/BulePrint/Core/Input/FB_BubbleBreak.FB_BubbleBreak" 0 "None" "0, 0, 0" "0, 0, 0" "KeepRelativeOffset" false false 1.0 0.0 0)))

(event Custom|BubbleBreak
  (params (CanDoubleJump :type Boolean))
  (bind _as_maincharacter (Variables|Default|GetAs%20Maincharacter))
  (if CanDoubleJump
    (Math|Integer|IncrementInt (Variables|/Script/Engine.Character|GetJumpMaxCount _as_maincharacter)
      (:%20%20
        (Character|StopJumping _as_maincharacter)
        (Character|Jump _as_maincharacter)
        (Actor|DestroyActor)))
    (else
      (CallFunction|SpawnSmall "1.000000,0.000000,0.000000"))))

(event Custom|SpawnSmall
  (params (Direction :type Vector))
  (bind _returnvalue (Transformation|GetActorTransform))
  (bind (_roll _pitch _yaw) (Math|Rotator|BreakRotator (.rotation _returnvalue)))
  (for _index (range 0 2)
    (Game|SpawnActorfromClass "/Game/Bubble/BulePrint/Core/BP_BubbleSmall.BP_BubbleSmall_C" (Math|Transform|MakeTransform (.location _returnvalue) (Math|Rotator|MakeRotator _roll (+ _pitch (* _index 15.0)) _yaw) "0.500000,0.500000,0.500000") "Undefined" "MultiplyWithRoot" 0 0))
  (Actor|DestroyActor))

(event EventBeginPlay
  (Actor|SetLifeSpan 3.0))

(fn ConstructionScript
  (Variables|/Script/Engine.ProjectileMovementComponent|SetInitialSpeed (Variables|Default|GetProjectileMovement) (Math|Float|SelectFloat (Variables|Default|GetChangedSpeed) (Variables|Default|GetDefaultSpeed) (Variables|Default|GetUseSpeed))))