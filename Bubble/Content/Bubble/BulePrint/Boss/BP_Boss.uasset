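; BP_Boss is an early prototype of a boss actor with health and placeholder skill events.
; Skill1_Bomb spawns a BossBullet at a randomized offset toward negative X from the boss and prints a debug message.
; Tick subtracts a fixed amount from Health every frame, with no check on the result.
; The other skills, Stage4 and ChangeStage are empty, and leftover stage and skill debug nodes are unconnected.
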(event Custom|Skill3_ChatDrop)

(event Custom|Skill1_Bomb
  (bind _returnvalue (Transformation|GetActorLocation))
  (bind (_x _y _z) (Math|Vector|BreakVector _returnvalue))
  (Game|SpawnActorfromClass "/Game/Bubble/BulePrint/Boss/BossBullet.BossBullet_C" (Math|Transform|MakeTransform (Math|Vector|MakeVector (- _x (Math|Random|RandomFloatinRange 2.8e+02 4.5e+02)) (+ _y (Math|Random|RandomFloatinRange -1e+02 1e+02)) _z) "0, 0, 0" "1.000000,1.000000,1.000000") "AdjustIfPossibleButAlwaysSpawn" "MultiplyWithRoot" 0 0)
  (Development|PrintString "skill1"))

(event Custom|Skill2_chatframe)

(event Custom|Stage4)

(event EventBeginPlay)

(event Collision|EventActorBeginOverlap
  (params (OtherActor :type Actor%20Object%20Reference)))

(event EventTick
  (params (DeltaSeconds :type Float%20%28single-precision%29))
  (Variables|Default|SetHealth (- (Variables|Default|GetHealth) 1e+01)))

(fn ConstructionScript)

(fn ChangeStage)