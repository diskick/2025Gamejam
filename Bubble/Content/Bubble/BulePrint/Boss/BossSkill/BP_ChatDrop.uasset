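; BP_ChatDrop is a boss skill hazard that shows a random Chinese chat-message sprite and drops toward the player.
; Each Tick compares X with the player; the first near match sets a downward velocity and gravity on its ProjectileMovement.
; Box overlaps send BeDamageMessage with zero damage to the other actor.
; The actor destroys itself below world Z zero; a lifespan call is left unconnected.
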(event OnComponentBeginOverlap(Box)
  (params (OverlappedComponent :type Primitive%20Component%20Object%20Reference) (OtherActor :type Actor%20Object%20Reference) (OtherComp :type Primitive%20Component%20Object%20Reference) (OtherBodyIndex :type Integer) (bFromSweep :type Boolean) (SweepResult :type Hit%20Result%20Structure%20%28by%20ref%29))
  (Class|Damage|BeDamage(Message) OtherActor 0.0 false))

(event EventBeginPlay
  (Rendering|Components|Sprite|SetSprite (Variables|Default|GetPaperSprite) (.OutItem (Utilities|Array|Random (Utilities|Array|MakeArray "/Game/Bubble/Asset/Texture/弹幕/什么都被你说了，别人说什么_Sprite.什么都被你说了，别人说什么_Sprite" "/Game/Bubble/Asset/Texture/弹幕/你看，又急了_Sprite.你看，又急了_Sprite" "/Game/Bubble/Asset/Texture/弹幕/听不进实话，你来plq就想_让人安慰你吧_Sprite.听不进实话，你来plq就想_让人安慰你吧_Sprite" "/Game/Bubble/Asset/Texture/弹幕/我说话难听，我先走了_Sprite.我说话难听，我先走了_Sprite" "/Game/Bubble/Asset/Texture/弹幕/组_1_Sprite.组_1_Sprite")))))

(event EventTick
  (params (DeltaSeconds :type Float%20%28single-precision%29))
  (bind _projectilemovement (Variables|Default|GetProjectileMovement))
  (if (Math|Float|NearlyEqual(Float) (.x (Transformation|GetActorLocation)) (.x (Transformation|GetActorLocation (Game|GetPlayerCharacter 0))) 1e+01)
    (Utilities|FlowControl|Sequence
      (:then_0
        (Utilities|FlowControl|DoOnce false
          (:Completed
            (Game|Components|ProjectileMovement|SetVelocityinLocalSpace _projectilemovement "0.000000,0.000000,-60.000000")
            (Variables|/Script/Engine.ProjectileMovementComponent|SetProjectileGravityScale _projectilemovement 0.3))))
      (:then_1
        (if (< (.z (Transformation|GetActorLocation)) 0.0) :!label _label
          (Actor|DestroyActor))))
    (else
      (goto _label))))

(fn ConstructionScript)